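; BP_JoustPlayerController is the player controller for jousting characters, keeping the camera's yaw within a limited arc around the pawn's facing.
; On possess, it casts the pawn to BP_JoustCharacter and caches the reference.
; Every tick it re-centers the PlayerCameraManager's min and max view yaw on the capsule's world yaw, offset by CameraYawLimit, so the allowed look range turns with the character.
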(event `self.ReceivePossess`
  (params (PossessedPawn :type "Pawn Object Reference"))
  (bind _asbp_joust_character (cast `/Game/Blueprints/BP_JoustCharacter` PossessedPawn))
  (set `self.Pawn Reference` _asbp_joust_character))

(event `self.ReceiveTick`
  (params (DeltaSeconds :type "Float (single-precision)"))
  (bind (_returnvalue_roll _returnvalue_pitch _returnvalue_yaw) (`KismetMathLibrary.BreakRotator` (`SceneComponent.K2_GetComponentRotation` (`Character.CapsuleComponent` (`self.Pawn Reference`)))))
  (set `PlayerCameraManager.ViewYawMin` (- _returnvalue_yaw (`self.CameraYawLimit`)) (`self.PlayerCameraManager`))
  (set `PlayerCameraManager.ViewYawMax` (+ _returnvalue_yaw (`self.CameraYawLimit`)) (`self.PlayerCameraManager`)))

(fn `UserConstructionScript`)