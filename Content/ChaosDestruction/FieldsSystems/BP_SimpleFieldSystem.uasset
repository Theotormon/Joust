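; BP_SimpleFieldSystem is a Chaos destruction field actor that applies strain and velocity to physics objects.
; Two seconds after BeginPlay, it applies external cluster strain through a radial falloff field with no falloff, sized and centered on its Sphere component.
; When a Pawn overlaps the sphere, it applies a radial linear velocity field, using the sweep impact normal as center position, and prints a debug "Hello".
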(event `self.ReceiveBeginPlay`
  (bind _sphere (`self.Sphere`))
  (`KismetSystemLibrary.Delay` 2.0)
  (`FieldSystemComponent.ApplyPhysicsField` (`self.FieldSystemComponent`) true "Field_ExternalClusterStrain" null (`RadialFalloff.SetRadialFalloff` (`self.RadialFalloff`) (`self.ExternalStrain`) 1.0 1.0 0.0 (`SphereComponent.GetScaledSphereRadius` _sphere) (`SceneComponent.K2_GetComponentLocation` _sphere) "Field_FallOff_None")))

(event `self.Sphere.OnComponentBeginOverlap`
  (params (OverlappedComponent :type "PrimitiveComponent Object Reference") (OtherActor :type "Actor Object Reference") (OtherComp :type "PrimitiveComponent Object Reference") (OtherBodyIndex :type Integer) (bFromSweep :type Boolean) (SweepResult :type "HitResult Structure (by ref)"))
  (cast `Pawn` OtherActor)
  (`FieldSystemComponent.ApplyPhysicsField` (`self.FieldSystemComponent`) true "Field_LinearVelocity" null (`RadialVector.SetRadialVector` (`self.RadialVector`) (`self.LinearVelocity`) (`.ImpactNormal` (`GameplayStatics.BreakHitResult` SweepResult))))
  (`KismetSystemLibrary.PrintString` "Hello"))

(fn `UserConstructionScript`)